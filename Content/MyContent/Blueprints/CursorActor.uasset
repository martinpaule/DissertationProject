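; CursorActor is a cursor actor that displays a spinning element which always faces the camera.
; On BeginPlay it caches the first CameraActor found in the level.
; Each tick it rolls PlaneRotator at SpinSpeed, scaled by delta time and negated.
; It also billboards the root by pointing its X axis at that camera's component location.
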(event EventBeginPlay
  (bind _returnvalue (Actor|GetActorOfClass "/Script/Engine.CameraActor"))
  (Variables|Default|SetCamRef _returnvalue))

(event Collision|EventActorBeginOverlap
  (params (OtherActor :type Actor%20Object%20Reference)))

(event EventTick
  (params (DeltaSeconds :type Float%20%28single-precision%29))
  (Transformation|AddRelativeRotation (Variables|Default|GetPlaneRotator) (Math|Rotator|MakeRotator (* DeltaSeconds (Variables|Default|GetSpinSpeed) -1.0) 0.0 0.0) false false)
  (Transformation|SetWorldRotation (Variables|Default|GetDefaultSceneRoot) (Math|Conversions|RotationFromXVector (Math|Vector|Normalize (- (Transformation|GetWorldLocation (Variables|/Script/Engine.CameraActor|GetCameraComponent (Variables|Default|GetCamRef))) (Transformation|GetActorLocation)))) false false))

(fn ConstructionScript)