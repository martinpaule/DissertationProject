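; DamageText is a floating damage number actor that shows a damage value in the world and destroys itself after a few seconds.
; InitializeVariables receives the damage, player reference and float direction, sets the text, picks a random float speed and changes the text color for higher damage tiers.
; Tick moves the actor along that direction and turns the text against the player's CameraAnchor forward vector, billboard style.
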(event EventBeginPlay)

(event Collision|EventActorBeginOverlap
  (params (OtherActor :type Actor%20Object%20Reference)))

(event EventTick
  (params (DeltaSeconds :type Float%20%28single-precision%29))
  (Variables|Default|SetLifeTime (- (Variables|Default|GetLifeTime) DeltaSeconds))
  (Transformation|SetWorldRotation (Variables|Default|GetTextRender) (Math|Conversions|RotationFromXVector (* (Math|Vector|GetForwardVector (Variables|/Game/MyContent/Blueprints/PlayerPawn.PlayerPawn_C|GetCameraAnchor (Variables|Default|GetPlayerRef))) -1.0)) false false)
  (Transformation|AddActorWorldOffset (* (* DeltaSeconds (Variables|Default|GetfloatSpeed)) (Variables|Default|GetfloatDirection)))
  (if (< (Variables|Default|GetLifeTime) 0.0)
    (Actor|DestroyActor)))

(fn ConstructionScript)

(fn InitializeVariables
  (params (Damage :type Integer) (Player%20Reference :type Player%20Pawn%20Object%20Reference) (FloatDirection :type Vector))
  (bind _textrender (Variables|Default|GetTextRender))
  (bind _output_get (Variables|Default|SetDamage Damage))
  (Variables|Default|SetPlayerRef Player%20Reference)
  (Variables|Default|SetfloatDirection FloatDirection)
  (Rendering|Components|TextRender|SetText (Variables|Default|GetTextRender) (Utilities|Text|ToText(String) (Utilities|String|ToString(Integer) _output_get)))
  (Variables|Default|SetfloatSpeed (Math|Random|RandomFloatinRange 5e+01 1e+02))
  (Variables|Default|SetLifeTime 3.0)
  (if (> (Variables|Default|GetDamage) 100)
    (if (> (Variables|Default|GetDamage) 200)
      (Rendering|Components|TextRender|SetTextRenderColor _textrender (Math|Color|MakeColor 255 0 0 255))
      (else
        (Rendering|Components|TextRender|SetTextRenderColor _textrender (Math|Color|MakeColor 255 255 0 255))))))