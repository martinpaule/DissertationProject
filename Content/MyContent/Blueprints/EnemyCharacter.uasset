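; Enemy character that takes damage from asteroids overlapping it and opens the end-game level when its health drops below zero.
; Damage scales with asteroid velocity, or player velocity if the asteroid is held, capped and shown by spawned floating damage text.
; The struck asteroid is hidden and flagged for destruction.
; Tick feeds zero velocity to movement animation, prints health, and keeps a text render offset from the enemy, turned toward the player's camera.
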(event EventBeginPlay
  (CallFunction|Initialize))

(event Collision|EventActorBeginOverlap
  (params (OtherActor :type Actor%20Object%20Reference))
  (CallFunction|HandleCollision OtherActor))

(event EventTick
  (params (DeltaSeconds :type Float%20%28single-precision%29))
  (CallFunction|UpdateAnims DeltaSeconds)
  (CallFunction|DrawDebugs)
  (CallFunction|UpdateHealth DeltaSeconds))

(fn ConstructionScript)

(fn DrawDebugs
  (Development|PrintString (Utilities|String|Append "Enemy Health:" (Utilities|String|ToString(Float) (Variables|Default|GetHealth))) true true "(R=0.000000,G=0.660000,B=1.000000,A=1.000000)" 0.0))

(fn UpdateAnims
  (params (DeltaTime :type Float%20%28double-precision%29))
  (Default|UpdateMovementAnims (Variables|Default|GetMyAnimationComponent) (Math|Vector|MakeVector 0.0 0.0 0.0) (Math|Float|MakeLiteralFloat 1e+02)))

(fn UpdateHealth
  (params (DeltaTime :type Float%20%28double-precision%29))
  (bind _returnvalue (Transformation|GetActorLocation))
  (bind _textrender (Variables|Default|GetTextRender))
  (bind _playerref (Variables|Default|GetPlayerRef))
  (bind _returnvalue_2 (Transformation|GetActorLocation _playerref))
  (bind _camera (Variables|/Game/MyContent/Blueprints/PlayerPawn.PlayerPawn_C|GetCamera _playerref))
  (bind _returnvalue_3 (Math|Vector|GetRightVector _camera))
  (bind _returnvalue_4 (- _returnvalue _returnvalue_2))
  (bind _returnvalue_5 (Math|Vector|Normalize _returnvalue_4))
  (bind _returnvalue_6 (Math|Vector|CrossProduct _returnvalue_5 _returnvalue_3))
  (bind _returnvalue_7 (Math|Vector|Normalize _returnvalue_6))
  (Transformation|SetWorldRotation _textrender (Math|Interpolation|RInterpTo (Transformation|GetWorldRotation (Variables|Default|GetTextRender)) (Transformation|GetWorldRotation (Variables|/Game/MyContent/Blueprints/PlayerPawn.PlayerPawn_C|GetCameraBackV (Variables|Default|GetPlayerRef))) DeltaTime 3e+01) false false)
  (Transformation|SetWorldLocation _textrender (+ (* _returnvalue_7 (Transformation|GetActorScale3D) "130.000000,130.000000,130.000000" (+ 0.5 (/ (Math|Float|Absolute(Float) (Math|Vector|DotProduct _returnvalue_7 (Math|Vector|GetUpVector (Variables|Character|GetMesh)))) 2.0))) _returnvalue) false false))

(fn Initialize
  (Variables|Default|SetHealth (Variables|Default|GetMaxHealth))
  (bind _returnvalue (Actor|GetActorOfClass "/Game/MyContent/Blueprints/PlayerPawn.PlayerPawn_C"))
  (Variables|Default|SetPlayerRef _returnvalue))

(fn HandleCollision
  (params (NewParam :type Actor%20Object%20Reference))
  (bind _playerref (Variables|Default|GetPlayerRef))
  (bind _floatingpawnmovement (Variables|/Game/MyContent/Blueprints/PlayerPawn.PlayerPawn_C|GetFloatingPawnMovement _playerref))
  (bind _velocity (Variables|/Script/Engine.MovementComponent|GetVelocity _floatingpawnmovement))
  (bind _returnvalue (Math|Vector|VectorLength _velocity))
  (bind _returnvalue_2 (/ _returnvalue 2.7e+02))
  (bind _returnvalue_3 (Math|Float|Clamp(Float) _returnvalue_2 0.0 5e+01))
  (bind _asasteroid (Utilities|Casting|CastToAsteroid NewParam))
  (bind _returnvalue_4 (Game|SpawnActorfromClass "/Game/MyContent/Blueprints/DamageText.DamageText_C" (Math|Transform|MakeTransform (+ (Transformation|GetActorLocation _asasteroid) (* (Math|Vector|Normalize (- (Transformation|GetActorLocation _asasteroid) (Transformation|GetActorLocation))) 5e+01)) "0, 0, 0" "10.000000,10.000000,10.000000") "AlwaysSpawn" 0 0))
  (if (!= (Variables|/Game/MyContent/Blueprints/PlayerPawn.PlayerPawn_C|GetholdingRef (Variables|Default|GetPlayerRef)) NewParam)
    (Variables|Default|SetHealth (- (Variables|Default|GetHealth) (Math|Float|Clamp(Float) (/ (Math|Vector|VectorLength (Variables|/Script/HonsProject.GravBodyComponent|Getvelocity (Variables|/Script/HonsProject.Asteroid|GetGravComp _asasteroid))) 1e+01) 0.0 5e+01)))
    (Default|InitializeVariables _returnvalue_4 (Math|Float|Truncate (Math|Float|Clamp(Float) (/ (Math|Vector|VectorLength (Variables|/Script/HonsProject.GravBodyComponent|Getvelocity (Variables|/Script/HonsProject.Asteroid|GetGravComp _asasteroid))) 1e+01) 0.0 5e+01)) _playerref (Math|Vector|Normalize (- (Transformation|GetActorLocation _asasteroid) (Transformation|GetActorLocation))))
    (else
      (Variables|Default|SetHealth (- (Variables|Default|GetHealth) _returnvalue_3))
      (Default|InitializeVariables _returnvalue_4 (Math|Float|Truncate _returnvalue_3) _playerref (Math|Vector|Normalize (- (Transformation|GetActorLocation _asasteroid) (Transformation|GetActorLocation))))))
  (Variables|/Script/HonsProject.GravBodyComponent|SettoBeDestroyed (Variables|/Script/HonsProject.Asteroid|GetGravComp _asasteroid) true)
  (Rendering|SetVisibility (Variables|/Script/HonsProject.Asteroid|GetStaticMeshComponent _asasteroid) false false)
  (Variables|/Script/Engine.Actor|SetbGenerateOverlapEventsDuringLevelStreaming _asasteroid false)
  (if (< (Variables|Default|GetHealth) 0.0)
    (Game|OpenLevel(byObjectReference) "/Game/Levels/EndGameUI.EndGameUI")))