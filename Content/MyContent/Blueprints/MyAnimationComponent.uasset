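; Animation component that computes blend values for a player pawn's locomotion and timed upper-body animations.
; Each tick, pawn speed sets a state value between 3 and 2, overwriting any timed lerp from SetAnimationTransfer.
; StartUpperBodyAnim begins a countdown that fades upper-body weight in and out over the first and last fifths and flags a mid-animation trigger.
; Tick also prints that weight as an integer for debugging.
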(event EventBeginPlay)

(event EventTick
  (params (DeltaSeconds :type Float%20%28single-precision%29))
  (CallFunction|UpdateAnimations DeltaSeconds)
  (CallFunction|UpdateMovementAnims)
  (Development|PrintString (Utilities|String|ToString(Integer) (Class|KismetMathLibrary|ToInt64(Float) (Variables|Default|GetupperBoduUSEAMOUNT)))))

(fn UpdateAnimations
  (params (DeltaTime :type Float%20%28double-precision%29))
  (CallFunction|UpdateUpperBodyAnims DeltaTime)
  (if (Variables|Default|GetChangingState)
    (if (< (- (.x (Variables|Default|GetTimeNowMax)) DeltaTime) 0.0)
      (Variables|Default|SetChangingState false)
      (Variables|Default|SetTimeNowMax (Math|Vector2D|MakeVector2D 0.0 (.y (Variables|Default|GetTimeNowMax))))
      (else
        (Variables|Default|SetTimeNowMax (Math|Vector2D|MakeVector2D (- (.x (Variables|Default|GetTimeNowMax)) DeltaTime) (.y (Variables|Default|GetTimeNowMax))))))
    (Variables|Default|SetStateOldGoalNow (Math|Vector|MakeVector (.x (Variables|Default|GetStateOldGoalNow)) (.y (Variables|Default|GetStateOldGoalNow)) (Math|Float|Lerp (.x (Variables|Default|GetStateOldGoalNow)) (.y (Variables|Default|GetStateOldGoalNow)) (- 1.0 (/ (.x (Variables|Default|GetTimeNowMax)) (.y (Variables|Default|GetTimeNowMax)))))))))

(fn SetAnimationTransfer
  (params (AnimA_position :type Float%20%28double-precision%29) (AnimB_position :type Float%20%28double-precision%29) (duration :type Float%20%28double-precision%29))
  (Variables|Default|SetTimeNowMax (Math|Vector2D|MakeVector2D duration duration))
  (Variables|Default|SetStateOldGoalNow (Math|Vector|MakeVector AnimA_position AnimB_position AnimA_position))
  (Variables|Default|SetChangingState true))

(fn UpdateMovementAnims
  (bind _playerref (Variables|Default|GetPlayerRef))
  (bind _floatingpawnmovement (Variables|/Game/MyContent/Blueprints/PlayerPawn.PlayerPawn_C|GetFloatingPawnMovement _playerref))
  (bind _maxspeed (Variables|/Script/Engine.FloatingPawnMovement|GetMaxSpeed _floatingpawnmovement))
  (Variables|Default|SetStateOldGoalNow (Math|Vector|MakeVector 0.0 0.0 (Math|Float|Lerp 3.0 2.0 (Math|Float|Clamp(Float) (/ (- (Math|Vector|VectorLength (Variables|/Script/Engine.MovementComponent|GetVelocity _floatingpawnmovement)) (/ _maxspeed 4.0)) (/ _maxspeed 2.0)))))))

(fn StartUpperBodyAnim
  (params (AnimToUse :type Float%20%28double-precision%29) (AnimationLifeTime :type Float%20%28double-precision%29) (TriggerAt :type Float%20%28double-precision%29))
  (Variables|Default|SetUpperAnimToUse AnimToUse)
  (Variables|Default|SetupperBoduUSEAMOUNT 1.0)
  (Variables|Default|SetUpperBodyLifeTime AnimationLifeTime)
  (Variables|Default|SetupperBodyTimeTrigger TriggerAt)
  (Variables|Default|SetAnimTriggerState 0)
  (Variables|Default|SetUpperBodyLifeTimeMax AnimationLifeTime)
  (Variables|Default|SetuseUpperBody true))

(fn UpdateUpperBodyAnims
  (params (DeltaTime :type Float%20%28double-precision%29))
  (if (Variables|Default|GetuseUpperBody)
    ;[1 1 1] Update Main decrementors
    (Variables|Default|SetupperBodyTimeTrigger (- (Variables|Default|GetupperBodyTimeTrigger) DeltaTime))
    (Variables|Default|SetUpperBodyLifeTime (- (Variables|Default|GetUpperBodyLifeTime) DeltaTime))
    ;[1 1 1] Trigger inside the animation
    (if (and (< (Variables|Default|GetupperBodyTimeTrigger) 0.0) (== (Variables|Default|GetAnimTriggerState) 0))
      (Variables|Default|SetAnimTriggerState 1))
    ;[1 1 1] Handle animation interpolation at the very start and end of adding upper body anim
    (if (< (/ (Variables|Default|GetUpperBodyLifeTime) (Variables|Default|GetUpperBodyLifeTimeMax)) 0.2)
      (Variables|Default|SetupperBoduUSEAMOUNT (* (/ (Variables|Default|GetUpperBodyLifeTime) (Variables|Default|GetUpperBodyLifeTimeMax)) 5.0)))
    (if (> (/ (Variables|Default|GetUpperBodyLifeTime) (Variables|Default|GetUpperBodyLifeTimeMax)) 0.8)
      (Variables|Default|SetupperBoduUSEAMOUNT (- 1.0 (* (- (/ (Variables|Default|GetUpperBodyLifeTime) (Variables|Default|GetUpperBodyLifeTimeMax)) 0.8) 5.0))))
    ;[1 1 1] Conditions for finishing upper body anim
    (if (< (Variables|Default|GetUpperBodyLifeTime) 0.0)
      (Variables|Default|SetupperBoduUSEAMOUNT 0.0)
      (Variables|Default|SetuseUpperBody false))))