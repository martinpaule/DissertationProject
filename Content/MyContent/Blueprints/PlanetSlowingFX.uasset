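; PlanetSlowingFX is an effect actor that follows a referenced asteroid, apparently as the marker of a temporary slowing effect.
; Each tick it counts down its lifetime and snaps to the asteroid's location.
; On expiry it resets the local time value on the asteroid's GravComp to normal and destroys itself; it also destroys itself if the asteroid reference becomes invalid.
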(event EventBeginPlay)

(event EventTick
  (params (DeltaSeconds :type Float%20%28single-precision%29))
  (Utilities|IsValid (Variables|Default|GetMyAsteroidRef)
    (:Is%20Valid
      (bind _output_get (Variables|Default|SetLifeTime (- (Variables|Default|GetLifeTime) DeltaSeconds)))
      (Transformation|SetActorLocation (Transformation|GetActorLocation (Variables|Default|GetMyAsteroidRef)) false false)
      (if (< _output_get 0.0)
        (Variables|/Script/HonsProject.GravBodyComponent|SetmyLocalTimeEditor (Variables|/Script/HonsProject.Asteroid|GetGravComp (Variables|Default|GetMyAsteroidRef)) 1.0)
        (Actor|DestroyActor :!label _label)))
    (:Is%20Not%20Valid
      (goto _label))))

(event Collision|EventActorBeginOverlap
  (params (OtherActor :type Actor%20Object%20Reference)))

(fn ConstructionScript)