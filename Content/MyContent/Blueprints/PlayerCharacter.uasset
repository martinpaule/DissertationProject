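; Player character Blueprint that carries an Asteroid found in the level and drives a timed animation transition value.
; BeginPlay grabs the Asteroid and starts a transition; every Tick snaps that actor to the mesh's RightHandIndex3 socket.
; SetAnimationTransfer stores start, goal and duration in vectors, and UpdateAnimations counts down each frame, linearly interpolating the current state until time runs out.
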(event EventBeginPlay
  (bind _returnvalue (Actor|GetActorOfClass "/Script/HonsProject.Asteroid"))
  (Variables|Default|SetholdingRef _returnvalue)
  (CallFunction|SetAnimationTransfer 0.0 2.0 2.0))

(event Collision|EventActorBeginOverlap
  (params (OtherActor :type Actor%20Object%20Reference)))

(event EventTick
  (params (DeltaSeconds :type Float%20%28single-precision%29))
  (CallFunction|UpdateAnimations DeltaSeconds)
  (Transformation|SetActorLocation (Variables|Default|GetholdingRef) (Transformation|GetSocketLocation (Variables|Character|GetMesh) "RightHandIndex3") false false))

(fn ConstructionScript)

(fn UpdateAnimations
  (params (DeltaTime :type Float%20%28double-precision%29))
  (if (Variables|Default|GetChangingState)
    (Variables|Default|SetTimeNowMax (Math|Vector|MakeVector (- (.x (Variables|Default|GetTimeNowMax)) DeltaTime) (.y (Variables|Default|GetTimeNowMax)) 0.0))
    (Variables|Default|SetStateOldGoalNow (Math|Vector|MakeVector (.x (Variables|Default|GetStateOldGoalNow)) (.y (Variables|Default|GetStateOldGoalNow)) (Math|Float|Lerp (.x (Variables|Default|GetStateOldGoalNow)) (.y (Variables|Default|GetStateOldGoalNow)) (- 1.0 (/ (.x (Variables|Default|GetTimeNowMax)) (.y (Variables|Default|GetTimeNowMax)))))))
    (if (< (.x (Variables|Default|GetTimeNowMax)) 0.0)
      (Variables|Default|SetChangingState false))))

(fn SetAnimationTransfer
  (params (AnimA_position :type Float%20%28double-precision%29) (AnimB_position :type Float%20%28double-precision%29) (duration :type Float%20%28double-precision%29))
  (Variables|Default|SetTimeNowMax (Math|Vector|MakeVector duration duration 0.0))
  (Variables|Default|SetStateOldGoalNow (Math|Vector|MakeVector AnimA_position AnimB_position AnimA_position))
  (Variables|Default|SetChangingState true))