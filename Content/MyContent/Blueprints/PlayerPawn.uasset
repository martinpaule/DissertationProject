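; Player pawn that flies through space, grabs and throws asteroids, and slows their local time with an expanding freeze sphere.
; Grab and throw wait for an animation component's trigger point, then remove or re-add the asteroid's gravity component in GameManager's body simulation.
; While held, the asteroid follows a hand socket; throws inherit pawn velocity.
; Tick grows the freeze sphere, restoring slowed asteroids once it overshoots its range.
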(event EventBeginPlay
  (Actor|DestroyActor (Game|Player|GetPlayerPawn 0))
  (Pawn|Possess (Game|GetPlayerController 0) self)
  (bind _returnvalue (Actor|GetActorOfClass "/Script/HonsProject.GameManager"))
  (bind _output_get (Variables|Default|SetGameManagerRef _returnvalue))
  (Class|GameManager|SpawnAsteroidat _output_get (/ (Transformation|GetActorLocation) 1e+03) "0, 0, 0" 1.0))

(event EventTick
  (params (DeltaSeconds :type Float%20%28single-precision%29))
  (CallFunction|HoldAsteroid)
  (CallFunction|ShowPickupText)
  (CallFunction|HandleDelayedAction)
  (Development|PrintString (Utilities|String|ToString(Float) (Math|Vector|VectorLength (Variables|/Script/Engine.MovementComponent|GetVelocity (Variables|Default|GetFloatingPawnMovement)))) true true "(R=0.000000,G=0.660000,B=1.000000,A=1.000000)" 0.0)
  (CallFunction|UpdateFreezeSkill))

(event Input|AxisEvents|InputAxisRotateRight
  (params (AxisValue :type Float%20%28single-precision%29))
  (Class|Actor|AddActorWorldRotation (* (Math|Conversions|RotationFromXVector (Class|KismetMathLibrary|VectorRight)) (* AxisValue (Utilities|Time|GetWorldDeltaSeconds)))))

(event Input|AxisEvents|InputAxisRotateUp
  (params (AxisValue :type Float%20%28single-precision%29))
  (Transformation|AddActorLocalRotation (* (Math|Conversions|RotationFromXVector (Math|Vector|VectorUp)) (* (Utilities|Time|GetWorldDeltaSeconds) AxisValue -1.0)) false false))

(event Input|ActionEvents|InputActionFreezeAroundMe
  (params (Key :type Key%20Structure :default "None"))
  (bind _freezesphere (Variables|Default|GetFreezeSphere))
  (:Pressed
    (if (not (Variables|Default|GetExpandingFreeze))
      (Variables|Default|SetExpandingFreeze true)
      (Transformation|SetWorldScale3D _freezesphere "0, 0, 0")
      (Rendering|SetVisibility _freezesphere true false))))

(event Input|ActionEvents|InputActionActionAction
  (params (Key :type Key%20Structure :default "None"))
  (:Pressed
    (CallFunction|LMBaction)))

(event Input|AxisEvents|InputAxisMoveForward
  (params (AxisValue :type Float%20%28single-precision%29))
  (Pawn|Input|AddMovementInput (Math|Vector|GetForwardVector (Variables|Default|GetCameraForwardV)) AxisValue false)
  (Default|HandleRotationOfPlayer (Variables|Default|GetMyCameraHandler) (> AxisValue 0.0)))

(event Input|AxisEvents|InputAxisMoveRight
  (params (AxisValue :type Float%20%28single-precision%29))
  (Pawn|Input|AddMovementInput (* AxisValue (Math|Vector|GetRightVector (Variables|Default|GetCameraForwardV))) 1.0 false))

(event Input|AxisEvents|InputAxisInteract
  (params (AxisValue :type Float%20%28single-precision%29)))

(event Input|AxisEvents|InputAxisLMBdown
  (params (AxisValue :type Float%20%28single-precision%29)))

(fn ConstructionScript
  (bind _self self)
  (Variables|/Game/MyContent/Blueprints/MyCameraHandler.MyCameraHandler_C|SetPlayerRef (Variables|Default|GetMyCameraHandler) _self)
  (Variables|/Game/MyContent/Blueprints/MyAnimationComponent.MyAnimationComponent_C|SetPlayerRef (Variables|Default|GetMyAnimationComponent) _self))

(fn HoldAsteroid
  (bind _holdingref (Variables|Default|GetholdingRef))
  (bind _mesh (Variables|Default|GetMesh))
  (bind _returnvalue (Transformation|GetSocketTransform _mesh "RightHandIndex3" "RTS_World"))
  ;[1 1 1] Update Asteroid position in player's hand
  (Utilities|IsValid _holdingref
    (:Is%20Valid
      (Transformation|SetActorTransform _holdingref (Math|Transform|MakeTransform (.location _returnvalue) (.rotation _returnvalue) (Transformation|GetActorScale3D _holdingref))))))

(fn LMBaction
  (bind _myanimationcomponent (Variables|Default|GetMyAnimationComponent))
  (Utilities|IsValid (Variables|Default|GetholdingRef)
    (:Is%20Valid
      ;[1 1 1] Start throwing asteroid
      (Default|StartUpperBodyAnim _myanimationcomponent 0.0 2.0 1.0)
      (Variables|Default|SetDelayedActionType "ThrowObject"))
    (:Is%20Not%20Valid
      ;[1 1 1] If there's something to grab, Start grabbing asteroid
      (if (> (Utilities|Array|Length (Collision|GetOverlappingActors (Variables|Default|GetInteractArea) "/Script/HonsProject.Asteroid" :!class /Script/Engine.PrimitiveComponent)) 0)
        (Default|StartUpperBodyAnim _myanimationcomponent 2.0 1.5 0.8)
        (Variables|Default|SetDelayedActionType "GrabObject")))))

(fn ShowPickupText
  ;[1 1 1] Prompt the user to pickup the asteroid
  (for _array_element (Collision|GetOverlappingActors (Variables|Default|GetInteractArea) "/Script/HonsProject.Asteroid" :!class /Script/Engine.PrimitiveComponent)
    (Rendering|Debug|DrawDebugString (Transformation|GetActorLocation _array_element) "Press 'E' to pickup" 0 "(R=1.000000,G=1.000000,B=1.000000,A=1.000000)")))

(fn HandleDelayedAction
  (bind _interactarea (Variables|Default|GetInteractArea))
  (bind _gamemanagerref (Variables|Default|GetGameManagerRef))
  (bind _myanimationcomponent (Variables|Default|GetMyAnimationComponent))
  (bind _overlappingactors (Collision|GetOverlappingActors _interactarea "/Script/HonsProject.Asteroid" :!class /Script/Engine.PrimitiveComponent))
  (bind _bodyhandler_ref (Variables|/Script/HonsProject.GameManager|GetBodyHandler_ref _gamemanagerref))
  (bind _mygravbodies (Variables|/Script/HonsProject.NBodyHandler|GetmyGravBodies _bodyhandler_ref))
  ;[1 1 1] Check if the animation reached its 'point of action'
  (if (== (Variables|/Game/MyContent/Blueprints/MyAnimationComponent.MyAnimationComponent_C|GetAnimTriggerState _myanimationcomponent) 1)
    (Variables|/Game/MyContent/Blueprints/MyAnimationComponent.MyAnimationComponent_C|SetAnimTriggerState _myanimationcomponent 2)
    (switch string (Variables|Default|GetDelayedActionType)
      (:GrabObject
        ;[1 1 1] grab the asteroid
        (if (> (Utilities|Array|Length _overlappingactors) 0)
          (bind _output_get (Variables|Default|SetholdingRef (.OutItem (Utilities|Array|Random _overlappingactors))))
          (bind _asasteroid (Utilities|Casting|CastToAsteroid _output_get))
          (Utilities|Array|RemoveItem _mygravbodies (Variables|/Script/HonsProject.Asteroid|GetGravComp _asasteroid))))
      (:ThrowObject
        (bind _asasteroid_2 (Utilities|Casting|CastToAsteroid (Variables|Default|GetholdingRef)))
        (Variables|/Script/HonsProject.GravBodyComponent|Setvelocity (Variables|/Script/HonsProject.Asteroid|GetGravComp _asasteroid_2) (+ (* (Math|Vector|GetForwardVector (Variables|Default|GetArrow)) 1e+02) (/ (Variables|/Script/Engine.MovementComponent|GetVelocity (Variables|Default|GetFloatingPawnMovement)) 25.0)))
        (Variables|/Script/HonsProject.GravBodyComponent|Setposition (Variables|/Script/HonsProject.Asteroid|GetGravComp _asasteroid_2) (/ (.location (Transformation|GetSocketTransform (Variables|Default|GetMesh) "RightHandIndex3" "RTS_World")) 1e+03))
        (Utilities|Array|Add _mygravbodies (Variables|/Script/HonsProject.Asteroid|GetGravComp _asasteroid_2))
        (Variables|Default|SetholdingRef 0)
        (Niagara|SpawnSystemAttached "/Game/MyContent/Graphics/PlanetRelated/p_Trail.p_Trail" (Variables|/Script/HonsProject.Asteroid|GetSceneComponent _asasteroid_2) "None" "0, 0, 0" "0, 0, 0" "KeepRelativeOffset" true)))))

(fn UpdateFreezeSkill
  (bind _freezesphere (Variables|Default|GetFreezeSphere))
  (if (Variables|Default|GetExpandingFreeze)
    ;[1 1 1] Update sphere size and material params
    (Transformation|SetWorldScale3D _freezesphere (+ (Transformation|GetWorldScale _freezesphere) (* (Math|Vector|MakeVector (Variables|Default|GetFreezeExpandSpeed) (Variables|Default|GetFreezeExpandSpeed) (Variables|Default|GetFreezeExpandSpeed)) (Utilities|Time|GetWorldDeltaSeconds))))
    (Rendering|Material|SetScalarParameterValueonMaterials _freezesphere "NumLines" (Math|Float|Lerp 3e+02 4.5e+02 (/ (.X (Math|Vector|BreakVector (Transformation|GetWorldScale (Variables|Default|GetFreezeSphere)))) (Variables|Default|GetFreezeRange))))
    ;[1 1 1] Loop through overlapped planets
    (for _array_element (Collision|GetOverlappingActors (Variables|Default|GetFreezeSphere) "/Script/HonsProject.Asteroid" :!class /Script/Engine.PrimitiveComponent)
      ;[1 1 1] Apply Time Slowed Down
      (bind _asasteroid (Utilities|Casting|CastToAsteroid _array_element))
      (if (== (Variables|/Script/HonsProject.GravBodyComponent|GetmyLocalTimeEditor (Variables|/Script/HonsProject.Asteroid|GetGravComp _asasteroid)) 1.0)
        (Variables|/Script/HonsProject.GravBodyComponent|SetmyLocalTimeEditor (Variables|/Script/HonsProject.Asteroid|GetGravComp _asasteroid) 0.1)
        (Utilities|Array|Add (Variables|Default|GetslowedDownPlanets) (Variables|/Script/HonsProject.Asteroid|GetGravComp _asasteroid))))
    (if (and (> (.X (Math|Vector|BreakVector (Transformation|GetWorldScale (Variables|Default|GetFreezeSphere)))) (Variables|Default|GetFreezeRange)) (Rendering|IsVisible (Variables|Default|GetFreezeSphere)))
      (Rendering|SetVisibility (Variables|Default|GetFreezeSphere) false false))
    ;[1 1 1] Remove slowdown of all planets
    (if (> (/ (.X (Math|Vector|BreakVector (Transformation|GetWorldScale (Variables|Default|GetFreezeSphere)))) (Variables|Default|GetFreezeRange)) 1.5)
      (for _array_element_2 (Variables|Default|GetslowedDownPlanets)
        (Variables|/Script/HonsProject.GravBodyComponent|SetmyLocalTimeEditor _array_element_2 1.0))
      (Variables|Default|SetExpandingFreeze false)
      (Transformation|SetWorldScale3D (Variables|Default|GetFreezeSphere) "0, 0, 0")
      (Utilities|Array|Clear (Variables|Default|GetslowedDownPlanets)))))