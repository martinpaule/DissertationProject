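; Enemy character that takes damage from asteroid impacts and opens the end-game level once its health drops below zero.
; Overlaps spawn an explosion and floating damage text, then hide the asteroid and flag it for destruction.
; Clamped damage scales with asteroid velocity, or player velocity if the player holds that asteroid.
; Tick feeds zero velocity to the animation component; camera-facing rotation, health-text placement and debug printing are disconnected.
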(event EventBeginPlay
  (CallFunction|Initialize))

(event Collision|EventActorBeginOverlap
  (params (OtherActor :type Actor%20Object%20Reference))
  (CallFunction|HandleCollision OtherActor))

(event EventTick
  (params (DeltaSeconds :type Float%20%28single-precision%29))
  (CallFunction|UpdateAnims DeltaSeconds)
  (CallFunction|DrawDebugs)
  (CallFunction|UpdateHealth DeltaSeconds))

(fn ConstructionScript)

(fn DrawDebugs)

(fn UpdateAnims
  (params (DeltaTime :type Float%20%28double-precision%29))
  (Default|UpdateMovementAnims (Variables|Default|GetMyAnimationComponent) (Math|Vector|MakeVector 0.0 0.0 0.0) (Math|Float|MakeLiteralFloat 1e+02)))

(fn UpdateHealth
  (params (DeltaTime :type Float%20%28double-precision%29)))

(fn Initialize
  (Variables|Default|SetHealth (Variables|Default|GetMaxHealth))
  (bind _returnvalue (Actor|GetActorOfClass "/Game/MyContent/Blueprints/PlayerPawn.PlayerPawn_C"))
  (Variables|Default|SetPlayerRef _returnvalue))

(fn HandleCollision
  (params (NewParam :type Actor%20Object%20Reference))
  (bind _playerref (Variables|Default|GetPlayerRef))
  (bind _floatingpawnmovement (Variables|/Game/MyContent/Blueprints/PlayerPawn.PlayerPawn_C|GetFloatingPawnMovement _playerref))
  (bind _velocity (Variables|/Script/Engine.MovementComponent|GetVelocity _floatingpawnmovement))
  (bind _returnvalue (Math|Vector|VectorLength _velocity))
  (bind _returnvalue_2 (/ _returnvalue 2.7e+02))
  (bind _returnvalue_3 (Math|Float|Clamp(Float) _returnvalue_2 0.0 5e+01))
  (bind _asasteroid (Utilities|Casting|CastToAsteroid NewParam))
  (Effects|SpawnEmitteratLocation "/Game/MyContent/Graphics/Particles/BH_Explosion.BH_Explosion" (Transformation|GetActorLocation _asasteroid) "0, 0, 0" "2.000000,2.000000,2.000000")
  (bind _returnvalue_4 (Game|SpawnActorfromClass "/Game/MyContent/Blueprints/DamageText.DamageText_C" (Math|Transform|MakeTransform (+ (Transformation|GetActorLocation _asasteroid) (* (Math|Vector|Normalize (- (Transformation|GetActorLocation _asasteroid) (Transformation|GetActorLocation))) 5e+01)) "0, 0, 0" "10.000000,10.000000,10.000000") "AlwaysSpawn" 0 0))
  (if (!= (Variables|/Game/MyContent/Blueprints/PlayerPawn.PlayerPawn_C|GetholdingRef (Variables|Default|GetPlayerRef)) NewParam)
    (Variables|Default|SetHealth (- (Variables|Default|GetHealth) (Math|Float|Clamp(Float) (/ (Math|Vector|VectorLength (Variables|/Script/HonsProject.GravBodyComponent|Getvelocity (Variables|/Script/HonsProject.Asteroid|GetGravComp _asasteroid))) 1e+01) 0.0 5e+01)))
    (Default|InitializeVariables _returnvalue_4 (Math|Float|Truncate (Math|Float|Clamp(Float) (/ (Math|Vector|VectorLength (Variables|/Script/HonsProject.GravBodyComponent|Getvelocity (Variables|/Script/HonsProject.Asteroid|GetGravComp _asasteroid))) 1e+01) 0.0 5e+01)) _playerref (Math|Vector|Normalize (- (Transformation|GetActorLocation _asasteroid) (Transformation|GetActorLocation))))
    (else
      (Variables|Default|SetHealth (- (Variables|Default|GetHealth) _returnvalue_3))
      (Default|InitializeVariables _returnvalue_4 (Math|Float|Truncate _returnvalue_3) _playerref (Math|Vector|Normalize (- (Transformation|GetActorLocation _asasteroid) (Transformation|GetActorLocation))))))
  (Variables|/Script/HonsProject.GravBodyComponent|SettoBeDestroyed (Variables|/Script/HonsProject.Asteroid|GetGravComp _asasteroid) true)
  (Rendering|SetVisibility (Variables|/Script/HonsProject.Asteroid|GetStaticMeshComponent _asasteroid) false false)
  (Variables|/Script/Engine.Actor|SetbGenerateOverlapEventsDuringLevelStreaming _asasteroid false)
  (if (< (Variables|Default|GetHealth) 0.0)
    (Game|OpenLevel(byObjectReference) "/Game/Levels/EndGameUI.EndGameUI")))