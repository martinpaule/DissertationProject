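; Camera handler that drives the player's CameraAnchor from the RMBdown input axis.
; Holding RMB orbits the anchor by mouse delta with clamped pitch; otherwise it eases toward the capsule's rotation once the player moves fast enough.
; HandleRotationOfPlayer, not called here, turns the player toward the camera while restoring the anchor's world rotation.
; Older offset-vector orbit logic remains as unexecuted nodes.
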(event EventBeginPlay
  (bind _output_get (Variables|Default|SetCam_Distance_Default 0.0))
  (Variables|Default|SetCam_Distance_Now _output_get))

(event EventTick
  (params (DeltaSeconds :type Float%20%28single-precision%29)))

(event Input|AxisEvents|InputAxisRMBdown
  (params (AxisValue :type Float%20%28single-precision%29))
  (CallFunction|HandleCameraRotation (> AxisValue 0.0)))

(fn HandleCameraRotation
  (params (RMBdown :type Boolean))
  (bind _returnvalue (Utilities|Time|GetWorldDeltaSeconds))
  (bind _returnvalue_2 (Game|GetPlayerController 0))
  (bind _playerref (Variables|Default|GetPlayerRef))
  (bind _camrotatespeed (Variables|Default|GetCamRotateSpeed))
  (bind _playerref_2 (Variables|Default|GetPlayerRef))
  (bind _playerref_3 (Variables|Default|GetPlayerRef))
  (bind (_deltax _deltay) (Class|PlayerController|GetInputMouseDelta _returnvalue_2))
  (bind _returnvalue_3 (* _returnvalue _camrotatespeed))
  (bind _cameraanchor (Variables|/Game/MyContent/Blueprints/PlayerPawn.PlayerPawn_C|GetCameraAnchor _playerref))
  (bind _cameraanchor_2 (Variables|/Game/MyContent/Blueprints/PlayerPawn.PlayerPawn_C|GetCameraAnchor _playerref_2))
  (bind _floatingpawnmovement (Variables|/Game/MyContent/Blueprints/PlayerPawn.PlayerPawn_C|GetFloatingPawnMovement _playerref_3))
  (bind _relativerotation (Variables|/Script/Engine.SceneComponent|GetRelativeRotation _cameraanchor_2))
  (if RMBdown
    ;[1 1 1] Apply camera dPos to the rotation of camera anchor
    (Transformation|SetRelativeRotation _cameraanchor_2 (Math|Rotator|MakeRotator (.roll _relativerotation) (Math|Float|Clamp(Float) (+ (* _deltay _returnvalue_3) (.pitch _relativerotation)) -88.0 88.0) (+ (* _deltax _returnvalue_3) (.yaw _relativerotation))) false false)
    (else
      ;[1 1 1] If the player is moving and not holding RMB, interpolate cam to the back of the player
      (if (> (/ (Math|Vector|VectorLength (Variables|/Script/Engine.MovementComponent|GetVelocity _floatingpawnmovement)) (Variables|/Script/Engine.FloatingPawnMovement|GetMaxSpeed _floatingpawnmovement)) 0.2)
        (Transformation|SetRelativeRotation _cameraanchor (Math|Interpolation|RInterpTo (Variables|/Script/Engine.SceneComponent|GetRelativeRotation _cameraanchor) (Variables|/Script/Engine.SceneComponent|GetRelativeRotation (Variables|/Game/MyContent/Blueprints/PlayerPawn.PlayerPawn_C|GetCapsule _playerref)) (Utilities|Time|GetWorldDeltaSeconds) 1.0) false false)))))

(fn HandleRotationOfPlayer
  (params (RmbDown :type Boolean))
  (bind _playerref (Variables|Default|GetPlayerRef))
  (bind _playerref_2 (Variables|Default|GetPlayerRef))
  (bind _cameraanchor (Variables|/Game/MyContent/Blueprints/PlayerPawn.PlayerPawn_C|GetCameraAnchor _playerref_2))
  (bind _returnvalue (Transformation|GetWorldRotation _cameraanchor))
  (if RmbDown
    (bind _output_get (Variables|/Game/MyContent/Blueprints/PlayerPawn.PlayerPawn_C|SetOldCamAnchorRot _playerref _returnvalue))
    (Transformation|SetActorRotation _playerref (Math|Interpolation|RInterpTo (Transformation|GetActorRotation _playerref_2) _returnvalue (Utilities|Time|GetWorldDeltaSeconds) 2.0))
    (Transformation|SetWorldRotation _cameraanchor _output_get false false)))