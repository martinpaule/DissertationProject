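; Skills component that casts an expanding sphere which slows the local time of Asteroid actors it overlaps.
; AttemptStartSkill starts the sphere if none is expanding and the Freeze cooldown is over.
; Tick counts down the cooldown and grows the sphere, scaling its material line count until it hides at max range.
; Slowed asteroids get a PlanetSlowingFX actor, noted to restore time on destroy; the skill-type switch is still empty.
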(event EventBeginPlay)

(event EventTick
  (params (DeltaSeconds :type Float%20%28single-precision%29))
  (CallFunction|UpdateSkill DeltaSeconds))

(fn UpdateSkill
  (params (DeltaTime :type Float%20%28double-precision%29))
  (bind _spellsphere (Variables|Default|GetSpellSphere))
  (CallFunction|UpdateSkillCD DeltaTime)
  (if (Variables|Default|GetExpandingSphere)
    ;[1 1 1] Update sphere size and material params
    (Transformation|SetWorldScale3D _spellsphere (+ (Transformation|GetWorldScale _spellsphere) (* (Math|Vector|MakeVector (Variables|Default|GetSphereExpandingSpeed) (Variables|Default|GetSphereExpandingSpeed) (Variables|Default|GetSphereExpandingSpeed)) DeltaTime)))
    (Rendering|Material|SetScalarParameterValueonMaterials _spellsphere "NumLines" (Math|Float|Lerp 3e+02 4.5e+02 (/ (.X (Math|Vector|BreakVector (Transformation|GetWorldScale (Variables|Default|GetSpellSphere)))) (Variables|Default|GetSphereRange))))
    ;[1 1 1] Loop through overlapped planets
    (for _array_element (Collision|GetOverlappingActors (Variables|Default|GetSpellSphere) "/Script/HonsProject.Asteroid" :!class /Script/Engine.PrimitiveComponent)
      (bind _asasteroid (Utilities|Casting|CastToAsteroid _array_element))
      (switch string (Variables|Default|GetSkillActive)
        (:Default
          _)
        (:Freeze
          _))
      ;[1 1 1] Apply Time Slowed Down -  particle effect will set time back on destroy
      (if (== (Variables|/Script/HonsProject.GravBodyComponent|GetmyLocalTimeEditor (Variables|/Script/HonsProject.Asteroid|GetGravComp _asasteroid)) 1.0)
        (Variables|/Script/HonsProject.GravBodyComponent|SetmyLocalTimeEditor (Variables|/Script/HonsProject.Asteroid|GetGravComp _asasteroid) 0.1)
        (bind _returnvalue (Game|SpawnActorfromClass "/Game/MyContent/Blueprints/PlanetSlowingFX.PlanetSlowingFX_C" (Math|Transform|MakeTransform "0, 0, 0" "0, 0, 0" "2.000000,2.000000,2.000000") "Undefined" _asasteroid 0))
        (Variables|/Game/MyContent/Blueprints/PlanetSlowingFX.PlanetSlowingFX_C|SetMyAsteroidRef _returnvalue _asasteroid)
        (Effects|SpawnEmitteratLocation "/Game/MyContent/Graphics/Particles/SkillCollideFX.SkillCollideFX" (Transformation|GetActorLocation _asasteroid) "0, 0, 0" "3.000000,3.000000,3.000000")))
    ;[1 1 1] Sphere expanding exit condition
    (if (and (> (.X (Math|Vector|BreakVector (Transformation|GetWorldScale (Variables|Default|GetSpellSphere)))) (Variables|Default|GetSphereRange)) (Rendering|IsVisible (Variables|Default|GetSpellSphere)))
      (Rendering|SetVisibility (Variables|Default|GetSpellSphere) false false)
      (Variables|Default|SetExpandingSphere false)
      (Transformation|SetWorldScale3D (Variables|Default|GetSpellSphere) "0, 0, 0"))))

(fn AttemptStartSkill
  (params (SkillToStart :type String))
  (bind _spellsphere (Variables|Default|GetSpellSphere))
  (if (and (not (Variables|Default|GetExpandingSphere)) (<= (Variables|Default|GetFreezeSkillCooldownNow) 0.0))
    (Variables|Default|SetSkillActive SkillToStart)
    (Variables|Default|SetExpandingSphere true)
    (Transformation|SetWorldScale3D _spellsphere "0, 0, 0")
    (Rendering|SetVisibility _spellsphere true false)
    (Variables|Default|SetFreezeSkillCooldownNow (Variables|Default|GetFreezeSkillCooldownMax))))

(fn UpdateSkillCD
  (params (DeltaTime :type Float%20%28double-precision%29))
  (if (> (Variables|Default|GetFreezeSkillCooldownNow) 0.0)
    (Variables|Default|SetFreezeSkillCooldownNow (- (Variables|Default|GetFreezeSkillCooldownNow) DeltaTime))))