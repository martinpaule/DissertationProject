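; PlanetName is a floating text label actor that follows its assigned planet and faces the camera.
; Every tick it moves above MyPlanet by the planet's vertical bounds extent plus a fixed margin.
; It finds the PlayerCameraManager actor at BeginPlay and turns its TextRender opposite that camera's forward vector, billboarding the text parallel to the view.
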(event EventBeginPlay
  (bind _returnvalue (Actor|GetActorOfClass "/Script/Engine.PlayerCameraManager"))
  (Variables|Default|SetPlayerRef _returnvalue))

(event Collision|EventActorBeginOverlap
  (params (OtherActor :type Actor%20Object%20Reference)))

(event EventTick
  (params (DeltaSeconds :type Float%20%28single-precision%29))
  (bind _myplanet (Variables|Default|GetMyPlanet))
  (Transformation|SetActorLocation (+ (Transformation|GetActorLocation _myplanet) (Math|Vector|MakeVector 0.0 0.0 (+ (.Z (Math|Vector|BreakVector (.BoxExtent (Collision|GetActorBounds _myplanet false false)))) 1.5e+02))) false false)
  (Transformation|SetWorldRotation (Variables|Default|GetTextRender) (Math|Conversions|RotationFromXVector (* (Math|Vector|GetForwardVector (Variables|/Script/Engine.PlayerCameraManager|GetTransformComponent (Variables|Default|GetPlayerRef))) -1.0)) false false))

(fn ConstructionScript)