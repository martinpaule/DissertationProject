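; Player pawn for space flight that moves relative to a camera anchor, picks up and throws asteroids, and triggers a Freeze skill.
; Grab and throw start upper-body animations; Tick polls their trigger point to run the delayed action.
; Held asteroids follow a hand socket and leave GameManager's gravity bodies until thrown back with added pawn velocity.
; Tick also shows debug pickup prompts and drives movement animations and speed-based warp particles.
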(event EventBeginPlay
  (Actor|DestroyActor (Game|Player|GetPlayerPawn 0))
  (Pawn|Possess (Game|GetPlayerController 0) self)
  (bind _returnvalue (Actor|GetActorOfClass "/Script/HonsProject.GameManager"))
  (Variables|Default|SetGameManagerRef _returnvalue)
  (Variables|/Game/MyContent/Blueprints/MySkillsComponent.MySkillsComponent_C|SetSpellSphere (Variables|Default|GetMySkillsComponent) (Variables|Default|GetFreezeSphere)))

(event EventTick
  (params (DeltaSeconds :type Float%20%28single-precision%29))
  (CallFunction|HoldAsteroid)
  (CallFunction|ShowPickupText)
  (CallFunction|UpdateAnimations))

(event Input|AxisEvents|InputAxisRotateRight
  (params (AxisValue :type Float%20%28single-precision%29))
  (Class|Actor|AddActorWorldRotation (* (Math|Conversions|RotationFromXVector (Class|KismetMathLibrary|VectorRight)) (* AxisValue (Utilities|Time|GetWorldDeltaSeconds)))))

(event Input|AxisEvents|InputAxisRotateUp
  (params (AxisValue :type Float%20%28single-precision%29))
  (Transformation|AddActorLocalRotation (* (Math|Conversions|RotationFromXVector (Math|Vector|VectorUp)) (* (Utilities|Time|GetWorldDeltaSeconds) AxisValue -1.0)) false false))

(event Input|ActionEvents|InputActionFreezeAroundMe
  (params (Key :type Key%20Structure))
  (:Pressed
    (Default|AttemptStartSkill (Variables|Default|GetMySkillsComponent) "Freeze")))

(event Input|ActionEvents|InputActionActionAction
  (params (Key :type Key%20Structure))
  (:Pressed
    (CallFunction|LMBaction)))

(event Input|AxisEvents|InputAxisMoveForward
  (params (AxisValue :type Float%20%28single-precision%29))
  (Pawn|Input|AddMovementInput (Math|Vector|GetForwardVector (Variables|Default|GetCameraAnchor)) AxisValue false)
  (Default|HandleRotationOfPlayer (Variables|Default|GetMyCameraHandler) (> AxisValue 0.0)))

(event Input|AxisEvents|InputAxisMoveRight
  (params (AxisValue :type Float%20%28single-precision%29))
  (Pawn|Input|AddMovementInput (Math|Vector|GetRightVector (Variables|Default|GetCameraAnchor)) AxisValue false))

(fn ConstructionScript
  (Variables|/Game/MyContent/Blueprints/MyCameraHandler.MyCameraHandler_C|SetPlayerRef (Variables|Default|GetMyCameraHandler) self))

(fn HoldAsteroid
  (bind _holdingref (Variables|Default|GetholdingRef))
  (bind _mesh (Variables|Default|GetMesh))
  (bind _returnvalue (Transformation|GetSocketTransform _mesh "RightHandIndex3" "RTS_World"))
  ;[1 1 1] Update Asteroid position in player's hand
  (Utilities|IsValid _holdingref
    (:Is%20Valid
      (Transformation|SetActorTransform _holdingref (Math|Transform|MakeTransform (.location _returnvalue) (.rotation _returnvalue) (Transformation|GetActorScale3D _holdingref))))))

(fn LMBaction
  (bind _myanimationcomponent (Variables|Default|GetMyAnimationComponent))
  (Utilities|IsValid (Variables|Default|GetholdingRef)
    (:Is%20Valid
      ;[1 1 1] Start throwing asteroid
      (Default|StartUpperBodyAnim _myanimationcomponent 0.0 2.0 1.0)
      (Variables|Default|SetDelayedActionType "ThrowObject"))
    (:Is%20Not%20Valid
      ;[1 1 1] If there's something to grab, Start grabbing asteroid
      (if (> (Utilities|Array|Length (Collision|GetOverlappingActors (Variables|Default|GetInteractArea) "/Script/HonsProject.Asteroid" :!class /Script/Engine.PrimitiveComponent)) 0)
        (Default|StartUpperBodyAnim _myanimationcomponent 2.0 1.5 0.8)
        (Variables|Default|SetDelayedActionType "GrabObject")))))

(fn ShowPickupText
  ;[1 1 1] Prompt the user to pickup the asteroid
  (for _array_element (Collision|GetOverlappingActors (Variables|Default|GetInteractArea) "/Script/HonsProject.Asteroid" :!class /Script/Engine.PrimitiveComponent)
    (Rendering|Debug|DrawDebugString (Transformation|GetActorLocation _array_element) "Press 'E/LMB' to pickup" 0 "(R=1.000000,G=1.000000,B=1.000000,A=1.000000)")))

(fn UpdateAnimations
  (bind _interactarea (Variables|Default|GetInteractArea))
  (bind _gamemanagerref (Variables|Default|GetGameManagerRef))
  (bind _myanimationcomponent (Variables|Default|GetMyAnimationComponent))
  (bind _overlappingactors (Collision|GetOverlappingActors _interactarea "/Script/HonsProject.Asteroid" :!class /Script/Engine.PrimitiveComponent))
  (CallFunction|UpdateFlyFX)
  ;[1 1 1] Check if the animation reached its 'point of action'
  (if (== (Variables|/Game/MyContent/Blueprints/MyAnimationComponent.MyAnimationComponent_C|GetAnimTriggerState _myanimationcomponent) 1)
    (Variables|/Game/MyContent/Blueprints/MyAnimationComponent.MyAnimationComponent_C|SetAnimTriggerState _myanimationcomponent 2)
    (switch string (Variables|Default|GetDelayedActionType)
      (:GrabObject
        ;[1 1 1] grab the asteroid
        (if (> (Utilities|Array|Length _overlappingactors) 0)
          (bind _output_get (Variables|Default|SetholdingRef (.OutItem (Utilities|Array|Random _overlappingactors))))
          (bind _asasteroid (Utilities|Casting|CastToAsteroid _output_get))
          (Class|GameManager|RemoveAsteroid _gamemanagerref (Variables|/Script/HonsProject.Asteroid|GetGravComp _asasteroid))))
      (:ThrowObject
        (Utilities|IsValid (Variables|Default|GetholdingRef)
          (:Is%20Valid
            (bind _asasteroid_2 (Utilities|Casting|CastToAsteroid (Variables|Default|GetholdingRef)))
            (Variables|/Script/HonsProject.GravBodyComponent|Setvelocity (Variables|/Script/HonsProject.Asteroid|GetGravComp _asasteroid_2) (+ (* (Math|Vector|GetForwardVector (Variables|Default|GetCapsule)) 1e+02) (/ (Variables|/Script/Engine.MovementComponent|GetVelocity (Variables|Default|GetFloatingPawnMovement)) 15.0)))
            (Variables|/Script/HonsProject.GravBodyComponent|Setposition (Variables|/Script/HonsProject.Asteroid|GetGravComp _asasteroid_2) (/ (.location (Transformation|GetSocketTransform (Variables|Default|GetMesh) "RightHandIndex3" "RTS_World")) 1e+03))
            (Class|GameManager|AddAsteroid _gamemanagerref (Variables|/Script/HonsProject.Asteroid|GetGravComp _asasteroid_2))
            (Variables|Default|SetholdingRef 0)
            (bind _returnvalue (Niagara|SpawnSystemAttached "/Game/MyContent/Graphics/Particles/p_Trail.p_Trail" (Variables|/Script/HonsProject.Asteroid|GetSceneComponent _asasteroid_2) "None" "0, 0, 0" "0, 0, 0" "KeepRelativeOffset" true))
            (Niagara|SetNiagaraVariable(LinearColor) _returnvalue "User.MyCol" (Utilities|Struct|MakeLinearColor 0.0 1.0 1.0 1.0))))))))

(fn UpdateFlyFX
  (bind _floatingpawnmovement (Variables|Default|GetFloatingPawnMovement))
  (bind _warpspeedparticles (Variables|Default|GetWarpSpeedParticles))
  (bind _warpspeedparticles_2 (Variables|Default|GetWarpSpeedParticles))
  (bind _warpspeedparticles_3 (Variables|Default|GetWarpSpeedParticles))
  (bind _returnvalue (Class|MovementComponent|GetMaxSpeed _floatingpawnmovement))
  (bind _returnvalue_2 (AssetData|GetAsset _warpspeedparticles_2))
  (bind _velocity (Variables|/Script/Engine.MovementComponent|GetVelocity _floatingpawnmovement))
  (bind _returnvalue_3 (Math|Vector|VectorLength _velocity))
  (bind _returnvalue_4 (== _returnvalue_2 "/Game/MyContent/Graphics/Particles/HyperSpaceFX.HyperSpaceFX"))
  (bind _returnvalue_5 (/ _returnvalue_3 _returnvalue))
  (bind _returnvalue_6 (- _returnvalue_5 0.5))
  (bind _returnvalue_7 (* _returnvalue_6 2.0))
  (Effects|Components|ParticleSystem|SetVectorParameter _warpspeedparticles_3 "ParticleMoveDir" (* _velocity _returnvalue_7 -3.0))
  (Effects|Components|ParticleSystem|SetFloatParameter _warpspeedparticles_3 "TrailLifeTime" _returnvalue_7)
  (Default|UpdateMovementAnims (Variables|Default|GetMyAnimationComponent) _velocity _returnvalue)
  (if (> _returnvalue_5 0.5)
    (if (not _returnvalue_4)
      (Class|NiagaraComponent|SetAsset _warpspeedparticles "/Game/MyContent/Graphics/Particles/HyperSpaceFX.HyperSpaceFX" true))
    (elif _returnvalue_4
      (Class|NiagaraComponent|SetAsset _warpspeedparticles 0 true))))